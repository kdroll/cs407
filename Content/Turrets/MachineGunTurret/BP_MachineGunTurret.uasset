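; Sentry turret that automatically fires blue laser projectiles at Enemy and EnemyTroll pawns until its ammo runs out.
; Pawn sensing adds living targets to a list, then turns the sentry toward the nearest valid entry unless disabled.
; Each firing cycle shoots main, left and right barrel sockets in sequence with muzzle flashes and delays, costing one ammo.
; A floating ammo counter yaws toward the player every tick.
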(event `self.ReceiveBeginPlay`
  ;[1 1 1] Ammo Count Initialization
  (set `self.CurrentAmmoCount` 100)
  (`TextRenderComponent.K2_SetText` (`self.AmmoCount`) (`KismetTextLibrary.Conv_IntToText` (`self.CurrentAmmoCount`))))

(event `self.PawnSensing.OnSeePawn`
  (params (Pawn :type "Pawn Object Reference"))
  (bind _enemiesinrange (`self.EnemiesInRange`))
  (bind _sentry (`self.Sentry`))
  ;[1 1 1] Aiming Logic
  (if (not (`self.Disabled`))
    (bind _asenemy (cast `/Game/TestEnemies/Enemy` Pawn)
      (:`then`
        (set `self.TargetIsDead` (`/Game/TestEnemies/Enemy.IsDead` _asenemy)))
      (:`CastFailed`
        (bind _asenemy_troll (cast `/Game/TestEnemies/EnemyTroll` Pawn))
        (set `self.TargetIsDead` (`/Game/TestEnemies/EnemyTroll.IsDead` _asenemy_troll))))
    (if (not (`self.TargetIsDead`))
      (if (not (`KismetArrayLibrary.Array_Contains` (`self.EnemiesInRange`) Pawn))
        (`KismetArrayLibrary.Array_Add` _enemiesinrange Pawn))
      (bind _returnednearestenemy (`self.GetNearestEnemy` _enemiesinrange))
      (`/Engine/EditorBlueprintResources/StandardMacros.IsValid` _returnednearestenemy
        (:`Is Valid`
          (`SceneComponent.K2_SetWorldRotation` _sentry (`KismetMathLibrary.MakeRotator` (* (.pitch (`KismetMathLibrary.FindLookAtRotation` (`SceneComponent.K2_GetComponentLocation` _sentry) (`self.K2_GetActorLocation` _returnednearestenemy))) -1.0) 0.0 (- (.yaw (`KismetMathLibrary.FindLookAtRotation` (`SceneComponent.K2_GetComponentLocation` _sentry) (`self.K2_GetActorLocation` _returnednearestenemy))) 90.0)) false false)
          (if (not (`self.CurrentlyFiring`))
            (`self.Shootenemy` _returnednearestenemy)))))))

(event `ShootEnemy`
  (params (Enemy :type "Pawn Object Reference"))
  ;[1 1 1] Shooting Logic
  (if (`self.Disabled`)
    _
    (elif (> (`self.CurrentAmmoCount`) 0)
      (set `self.CurrentlyFiring` true)
      (`|SpawnActorFromClass` "/Game/FirstPersonBP/Blueprints/LaserBeamProjectile_Blue.LaserBeamProjectile_Blue_C" (`SceneComponent.GetSocketTransform` (`self.Sentry`) "MainBarrel" "RTS_World") "AdjustIfPossibleButDontSpawnIfColliding" "OverrideRootScale")
      (`GameplayStatics.SpawnEmitterAtLocation` "/Game/InfinityBladeEffects/Effects/FX_Monsters/FX_Monster_Gruntling/Master/LaserMuzzleFlash.LaserMuzzleFlash" (`SceneComponent.GetSocketLocation` (`self.Sentry`) "MainBarrelEffect"))
      (`KismetSystemLibrary.Delay` (`self.FireInterval`))
      (`|SpawnActorFromClass` "/Game/FirstPersonBP/Blueprints/LaserBeamProjectile_Blue.LaserBeamProjectile_Blue_C" (`SceneComponent.GetSocketTransform` (`self.Sentry`) "LeftBarrel" "RTS_World") "AdjustIfPossibleButDontSpawnIfColliding" "OverrideRootScale")
      (`GameplayStatics.SpawnEmitterAtLocation` "/Game/InfinityBladeEffects/Effects/FX_Monsters/FX_Monster_Gruntling/Master/LaserMuzzleFlash.LaserMuzzleFlash" (`SceneComponent.GetSocketLocation` (`self.Sentry`) "LeftBarrelEffect"))
      (`KismetSystemLibrary.Delay` (`self.FireInterval`))
      (`|SpawnActorFromClass` "/Game/FirstPersonBP/Blueprints/LaserBeamProjectile_Blue.LaserBeamProjectile_Blue_C" (`SceneComponent.GetSocketTransform` (`self.Sentry`) "RightBarrel" "RTS_World") "Undefined" "OverrideRootScale")
      (`GameplayStatics.SpawnEmitterAtLocation` "/Game/InfinityBladeEffects/Effects/FX_Monsters/FX_Monster_Gruntling/Master/LaserMuzzleFlash.LaserMuzzleFlash" (`SceneComponent.GetSocketLocation` (`self.Sentry`) "RightBarrelEffect"))
      (`KismetSystemLibrary.Delay` (`self.FireInterval`))
      (`/Engine/EditorBlueprintResources/StandardMacros.DecrementInt` (`self.CurrentAmmoCount`)
        (:`  `
          (`TextRenderComponent.K2_SetText` (`self.AmmoCount`) (`KismetTextLibrary.Conv_IntToText` (`self.CurrentAmmoCount`)))
          (set `self.CurrentlyFiring` false))))))

(event `self.ReceiveTick`
  (params (DeltaSeconds :type "Float (single-precision)"))
  (bind _ammocount (`self.AmmoCount`))
  ;[1 1 1] Ammo Count Display Logic
  (`SceneComponent.K2_SetWorldRotation` _ammocount (`KismetMathLibrary.MakeRotator` 0.0 0.0 (.yaw (`KismetMathLibrary.FindLookAtRotation` (`SceneComponent.K2_GetComponentLocation` _ammocount) (`self.K2_GetActorLocation` (`GameplayStatics.GetPlayerCharacter` 0))))) false false))

(fn `GetNearestEnemy`
  (params (EnemiesInRange :type "Array of Pawn Object Reference (by ref)"))
  (returns (ReturnedNearestEnemy :type "Pawn Object Reference"))
  (set `self.ShortestDistance` 100000000.0)
  (for (_array_element _array_index) EnemiesInRange
    (`/Engine/EditorBlueprintResources/StandardMacros.IsValid` _array_element
      (:`Is Valid`
        (bind _returnvalue (`self.GetDistanceTo` _array_element))
        (if (< _returnvalue (`self.ShortestDistance`))
          (set `self.ShortestDistance` _returnvalue)
          (set `self.NearestEnemy` _array_element)))
      (:`Is Not Valid`
        (`KismetArrayLibrary.Array_Remove` EnemiesInRange _array_index))))
  (return (`self.NearestEnemy`)))

(fn `UserConstructionScript`)
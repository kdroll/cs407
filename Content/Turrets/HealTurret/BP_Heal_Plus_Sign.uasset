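; BP_Heal_Plus_Sign is a short-lived floating plus-sign actor for the Heal Turret.
; On BeginPlay it caches its spawn location and plays a timeline whose scaled Height track offsets it vertically.
; Each timeline update also turns it to face the first player's pawn, with pitch locked to zero.
; The actor destroys itself when the timeline finishes.
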(event `self.ReceiveBeginPlay`
  (bind (_startinglocation_x _startinglocation_y _startinglocation_z) (`KismetMathLibrary.BreakVector` (`self.StartingLocation`)))
  (set `self.StartingLocation` (`self.K2_GetActorLocation`))
  (bind (_direction _opacity _height) (`Timeline|Animation`)
    (:`Update`
      (`self.K2_SetActorLocationAndRotation` (`KismetMathLibrary.MakeVector` _startinglocation_x _startinglocation_y (+ _startinglocation_z (* _height 100.0))) (`KismetMathLibrary.MakeRotator` (.roll (`KismetMathLibrary.FindLookAtRotation` (`self.K2_GetActorLocation`) (`self.K2_GetActorLocation` (`GameplayStatics.GetPlayerPawn` 0)))) 0.0 (.yaw (`KismetMathLibrary.FindLookAtRotation` (`self.K2_GetActorLocation`) (`self.K2_GetActorLocation` (`GameplayStatics.GetPlayerPawn` 0)))))))
    (:`Finished`
      (`self.K2_DestroyActor`))))

(fn `UserConstructionScript`)
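; BP_SlowTower is a turret that slows Enemy and EnemyTroll actors inside its SlowSphere while it has ammo.
; Sphere entry sets the enemy's CustomTimeDilation to SlowFactor and spends one ammo; exit restores it to 1.0.
; Overlaps also maintain an in-range enemy count, which this graph never reads.
; Tick yaws the ammo text toward the player and spins the model by a fixed, frame-rate-dependent step.
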(event `self.ReceiveTick`
  (params (DeltaSeconds :type "Float (single-precision)"))
  (bind _slowturretmodel (`self.SlowTurretModel`))
  (bind _ammocount (`self.AmmoCount`))
  ;[1 1 1] Ammo Count Display Logic
  (`SceneComponent.K2_SetWorldRotation` _ammocount (`KismetMathLibrary.MakeRotator` 0.0 0.0 (.yaw (`KismetMathLibrary.FindLookAtRotation` (`SceneComponent.K2_GetComponentLocation` _ammocount) (`self.K2_GetActorLocation` (`GameplayStatics.GetPlayerCharacter` 0))))) false false)
  ;[1 1 1] Rotation Logic
  (`SceneComponent.K2_SetWorldRotation` _slowturretmodel (`KismetMathLibrary.MakeRotator` (.roll (`SceneComponent.K2_GetComponentRotation` _slowturretmodel)) (.pitch (`SceneComponent.K2_GetComponentRotation` _slowturretmodel)) (+ (.yaw (`SceneComponent.K2_GetComponentRotation` _slowturretmodel)) 0.1)) false false))

(event `self.SlowSphere.OnComponentBeginOverlap`
  (params (OverlappedComponent :type "PrimitiveComponent Object Reference") (OtherActor :type "Actor Object Reference") (OtherComp :type "PrimitiveComponent Object Reference") (OtherBodyIndex :type Integer) (bFromSweep :type Boolean) (SweepResult :type "HitResult Structure (by ref)"))
  ;[1 1 1] Slow Enemy Detection Logic
  (bind _asenemy (cast `/Game/TestEnemies/Enemy` OtherActor)
    (:`then`
      (`/Engine/EditorBlueprintResources/StandardMacros.IncrementInt` (`self.NumEnemiesInSlowSphere`)
        (:`  `
          (`self.SlowEnemy` _asenemy))))
    (:`CastFailed`
      (bind _asenemy_troll (cast `/Game/TestEnemies/EnemyTroll` OtherActor))
      (`/Engine/EditorBlueprintResources/StandardMacros.IncrementInt` (`self.NumEnemiesInSlowSphere`)
        (:`  `
          (`self.SlowEnemy` _asenemy_troll))))))

(event `self.ReceiveBeginPlay`
  ;[1 1 1] Initialize Ammo Count
  (set `self.CurrentAmmoCount` (`self.InitialAmmo`))
  (`TextRenderComponent.K2_SetText` (`self.AmmoCount`) (`KismetTextLibrary.Conv_IntToText` (`self.CurrentAmmoCount`))))

(event `self.SlowSphere.OnComponentEndOverlap`
  (params (OverlappedComponent :type "PrimitiveComponent Object Reference") (OtherActor :type "Actor Object Reference") (OtherComp :type "PrimitiveComponent Object Reference") (OtherBodyIndex :type Integer))
  ;[1 1 1] Slow Enemy Detection Logic
  (bind _asenemy (cast `/Game/TestEnemies/Enemy` OtherActor)
    (:`then`
      (`/Engine/EditorBlueprintResources/StandardMacros.DecrementInt` (`self.NumEnemiesInSlowSphere`)
        (:`  `
          (`self.RemoveSlowFromEnemy` _asenemy))))
    (:`CastFailed`
      (bind _asenemy_troll (cast `/Game/TestEnemies/EnemyTroll` OtherActor))
      (`/Engine/EditorBlueprintResources/StandardMacros.DecrementInt` (`self.NumEnemiesInSlowSphere`)
        (:`  `
          (`self.RemoveSlowFromEnemy` _asenemy_troll))))))

(fn `RemoveSlowFromEnemy`
  (params (EnemyReference :type "Actor Object Reference"))
  (set `Actor.CustomTimeDilation` 1.0 EnemyReference))

(fn `SlowEnemy`
  (params (EnemyReference :type "Actor Object Reference"))
  (bind _currentammocount (`self.CurrentAmmoCount`))
  (if (> (`self.CurrentAmmoCount`) 0)
    (set `Actor.CustomTimeDilation` (`self.SlowFactor`) EnemyReference)
    (`/Engine/EditorBlueprintResources/StandardMacros.DecrementInt` _currentammocount
      (:`  `
        (`TextRenderComponent.K2_SetText` (`self.AmmoCount`) (`KismetTextLibrary.Conv_IntToText` _currentammocount))))))

(fn `UserConstructionScript`)
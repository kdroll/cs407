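; Test sentry turret that automatically aims and fires lasers at Enemy and EnemyTroll pawns.
; PawnSensing sightings add pawns to EnemiesInRange, then GetNearestEnemy picks the closest valid one and drops invalid entries.
; The Sentry mesh snaps toward that target with an axis-corrected look-at rotation.
; Unless already firing, it spawns blue laser projectiles and muzzle flashes from three barrel sockets in sequence, spaced by FireInterval.
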(event `self.PawnSensing.OnSeePawn`
  (params (Pawn :type "Pawn Object Reference"))
  (bind _enemiesinrange (`self.EnemiesInRange`))
  (bind _sentry (`self.Sentry`))
  ;[1 1 1] Aiming Logic
  (cast `/Game/TestEnemies/Enemy` Pawn
    (:`then`
      _)
    (:`CastFailed`
      (cast `/Game/TestEnemies/EnemyTroll` Pawn)))
  (if (not (`KismetArrayLibrary.Array_Contains` (`self.EnemiesInRange`) Pawn))
    (`KismetArrayLibrary.Array_Add` _enemiesinrange Pawn))
  (bind _returnedclosestenemy (`self.GetNearestEnemy` _enemiesinrange))
  (`/Engine/EditorBlueprintResources/StandardMacros.IsValid` _returnedclosestenemy
    (:`Is Valid`
      (`SceneComponent.K2_SetWorldRotation` _sentry (`KismetMathLibrary.MakeRotator` (* (.pitch (`KismetMathLibrary.FindLookAtRotation` (`SceneComponent.K2_GetComponentLocation` _sentry) (`self.K2_GetActorLocation` _returnedclosestenemy))) -1.0) 0.0 (- (.yaw (`KismetMathLibrary.FindLookAtRotation` (`SceneComponent.K2_GetComponentLocation` _sentry) (`self.K2_GetActorLocation` _returnedclosestenemy))) 90.0)) false false)
      (if (not (`self.CurrentlyFiring`))
        (`self.Shootenemy` _returnedclosestenemy)))))

(event `ShootEnemy`
  (params (Enemy :type "Pawn Object Reference"))
  (bind _returnvalue (`SceneComponent.GetSocketTransform` (`self.Sentry`) "RightBarrel" "RTS_World"))
  (bind _returnvalue_2 (`SceneComponent.GetSocketTransform` (`self.Sentry`) "MainBarrel" "RTS_World"))
  (bind _returnvalue_3 (`SceneComponent.GetSocketTransform` (`self.Sentry`) "LeftBarrel" "RTS_World"))
  ;[1 1 1] Shooting Logic
  (set `self.CurrentlyFiring` true)
  (`|SpawnActorFromClass` "/Game/FirstPersonBP/Blueprints/LaserBeamProjectile_Blue.LaserBeamProjectile_Blue_C" _returnvalue_2 "AdjustIfPossibleButDontSpawnIfColliding" "OverrideRootScale")
  (`GameplayStatics.SpawnEmitterAtLocation` "/Game/InfinityBladeEffects/Effects/FX_Monsters/FX_Monster_Gruntling/Master/LaserMuzzleFlash.LaserMuzzleFlash" (`KismetMathLibrary.TransformLocation` _returnvalue_2))
  (`KismetSystemLibrary.Delay` (`self.FireInterval`))
  (`|SpawnActorFromClass` "/Game/FirstPersonBP/Blueprints/LaserBeamProjectile_Blue.LaserBeamProjectile_Blue_C" _returnvalue_3 "AdjustIfPossibleButDontSpawnIfColliding" "OverrideRootScale")
  (`GameplayStatics.SpawnEmitterAtLocation` "/Game/InfinityBladeEffects/Effects/FX_Monsters/FX_Monster_Gruntling/Master/LaserMuzzleFlash.LaserMuzzleFlash" (`KismetMathLibrary.TransformLocation` _returnvalue_3))
  (`KismetSystemLibrary.Delay` (`self.FireInterval`))
  (`|SpawnActorFromClass` "/Game/FirstPersonBP/Blueprints/LaserBeamProjectile_Blue.LaserBeamProjectile_Blue_C" _returnvalue "Undefined" "OverrideRootScale")
  (`GameplayStatics.SpawnEmitterAtLocation` "/Game/InfinityBladeEffects/Effects/FX_Monsters/FX_Monster_Gruntling/Master/LaserMuzzleFlash.LaserMuzzleFlash" (`KismetMathLibrary.TransformLocation` _returnvalue))
  (`KismetSystemLibrary.Delay` (`self.FireInterval`))
  (set `self.CurrentlyFiring` false))

(fn `GetNearestEnemy`
  (params (EnemiesInRange :type "Array of Pawn Object Reference (by ref)"))
  (returns (ReturnedClosestEnemy :type "Pawn Object Reference"))
  (set `self.ShortestDistance` 100000000.0)
  (for (_array_element _array_index) EnemiesInRange
    (`/Engine/EditorBlueprintResources/StandardMacros.IsValid` _array_element
      (:`Is Valid`
        (bind _returnvalue (`self.GetDistanceTo` _array_element))
        (if (< _returnvalue (`self.ShortestDistance`))
          (set `self.ShortestDistance` _returnvalue)
          (set `self.ClosestEnemy` _array_element)))
      (:`Is Not Valid`
        (`KismetArrayLibrary.Array_Remove` EnemiesInRange _array_index))))
  (return (`self.ClosestEnemy`)))

(fn `UserConstructionScript`)
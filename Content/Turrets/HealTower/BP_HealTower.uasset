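; Heal tower turret that restores health to a player inside its HealSphere, spending displayed ammo per heal.
; Overlap events flag the player, and Tick uses Delays to pace HealPlayer and random plus-sign spawns.
; Tick also spins the tower, turns the ammo text toward the player and applies upgrade flags.
; Upgrades widen range, raise healing, halve ammo use, or damage-boost the player while in range (Juggernaut).
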(event `self.ReceiveBeginPlay`
  ;[1 1 1] Update Ammo Count Display
  (set `self.CurrentAmmoCount` (`self.InitialAmmo`))
  (`TextRenderComponent.K2_SetText` (`self.AmmoCount`) (`KismetTextLibrary.Conv_IntToText` (`self.CurrentAmmoCount`)))
  (set `self.FirstPersonCharacterReference` (`GameplayStatics.GetPlayerCharacter` 0)))

(event `self.ReceiveTick`
  (params (DeltaSeconds :type "Float (single-precision)"))
  (bind _st_tower (`self.ST_Tower`))
  (bind _ammocount (`self.AmmoCount`))
  ;[1 1 1] Check for Juggernaut Upgrade
  (bind _asfirst_person_character (cast `/Game/FirstPersonBP/Blueprints/FirstPersonCharacter` (`self.FirstPersonCharacterReference`))
    (:`then`
      (if (and (`self.Level3UpgradeIsJuggernaut`) (`self.HealIsOverlappingPlayer`))
        (`KismetSystemLibrary.PrintString` "yes")
        (set `/Game/FirstPersonBP/Blueprints/FirstPersonCharacter.IsDamageBoosted` true _asfirst_person_character)
        (else
          (`KismetSystemLibrary.PrintString` "no")
          (set `/Game/FirstPersonBP/Blueprints/FirstPersonCharacter.IsDamageBoosted` false _asfirst_person_character))))
    (:`CastFailed`
      _))
  ;[1 1 1] Check for Range Upgrade
  (if (`self.Level2UpgradeIsRange`)
    (`SceneComponent.SetRelativeScale3D` (`self.HealSphere`) (`self.UpgradedRangeVector`)))
  ;[1 1 1] Check for Power Upgrade
  (if (`self.Level2UpgradeIsPower`)
    (set `self.HealAmount` (`self.UpgradedHealAmount`)))
  ;[1 1 1] Ammo Count Display Logic
  (`SceneComponent.K2_SetWorldRotation` _ammocount (`KismetMathLibrary.MakeRotator` 0.0 0.0 (.yaw (`KismetMathLibrary.FindLookAtRotation` (`SceneComponent.K2_GetComponentLocation` _ammocount) (`self.K2_GetActorLocation` (`GameplayStatics.GetPlayerCharacter` 0))))) false false)
  ;[1 1 1] Rotation Logic
  (`SceneComponent.K2_SetWorldRotation` _st_tower (`KismetMathLibrary.MakeRotator` (.roll (`SceneComponent.K2_GetComponentRotation` _st_tower)) (.pitch (`SceneComponent.K2_GetComponentRotation` _st_tower)) (+ (.yaw (`SceneComponent.K2_GetComponentRotation` _st_tower)) 0.1)) false false)
  ;[1 1 1] Spawn Heal Signs
  (`KismetSystemLibrary.Delay` 0.4)
  (`|SpawnActorFromClass` "/Game/Turrets/HealTower/BP_Heal_Plus_Sign.BP_Heal_Plus_Sign_C" (`KismetMathLibrary.MakeTransform` (`KismetMathLibrary.MakeVector` (+ (.x (`SceneComponent.K2_GetComponentLocation` (`self.DefaultSceneRoot`))) (`KismetMathLibrary.RandomFloatInRange` -100.0 100.0)) (+ (.y (`SceneComponent.K2_GetComponentLocation` (`self.DefaultSceneRoot`))) (`KismetMathLibrary.RandomFloatInRange` -100.0 100.0)) (+ (.z (`SceneComponent.K2_GetComponentLocation` (`self.DefaultSceneRoot`))) (`KismetMathLibrary.RandomFloatInRange` 50.0 260.0)))) "Undefined" "OverrideRootScale")
  ;[1 1 1] Heal Player
  (if (`self.HealIsOverlappingPlayer`)
    (`KismetSystemLibrary.Delay` 1.0)
    (`self.HealPlayer` (`self.OverlappingPlayerReference`))))

(event `self.HealSphere.OnComponentBeginOverlap`
  (params (OverlappedComponent :type "PrimitiveComponent Object Reference") (OtherActor :type "Actor Object Reference") (OtherComp :type "PrimitiveComponent Object Reference") (OtherBodyIndex :type Integer) (bFromSweep :type Boolean) (SweepResult :type "HitResult Structure (by ref)"))
  ;[1 1 1] Heal Player Logic
  (bind _asfirst_person_character (cast `/Game/FirstPersonBP/Blueprints/FirstPersonCharacter` OtherActor))
  (set `self.HealIsOverlappingPlayer` true)
  (set `self.OverlappingPlayerReference` _asfirst_person_character))

(event `self.HealSphere.OnComponentEndOverlap`
  (params (OverlappedComponent :type "PrimitiveComponent Object Reference") (OtherActor :type "Actor Object Reference") (OtherComp :type "PrimitiveComponent Object Reference") (OtherBodyIndex :type Integer))
  ;[1 1 1] Heal Player Logic
  (set `self.HealIsOverlappingPlayer` false))

(fn `HealPlayer`
  (params (`Player Reference` :type "Actor Object Reference"))
  (bind _currentammocount (`self.CurrentAmmoCount`))
  (bind _currentammocount_2 (`self.CurrentAmmoCount`))
  (bind _asfirst_person_character (cast `/Game/FirstPersonBP/Blueprints/FirstPersonCharacter` `Player Reference`))
  ;[1 1 1] Check to see if ammo > 0
  (if (> (`self.CurrentAmmoCount`) 0)
    ;[1 1 1] Make sure health isn't currently at max
    (if (not (== (`/Game/FirstPersonBP/Blueprints/FirstPersonCharacter.Health` _asfirst_person_character) (`/Game/FirstPersonBP/Blueprints/FirstPersonCharacter.MaxHealth` _asfirst_person_character)))
      (bind _returnvalue (+ (`/Game/FirstPersonBP/Blueprints/FirstPersonCharacter.Health` _asfirst_person_character) (`self.HealAmount`)))
      (bind _maxhealth (`/Game/FirstPersonBP/Blueprints/FirstPersonCharacter.MaxHealth` _asfirst_person_character))
      ;[1 1 1] Make sure health doesn't exceed max
      (if (> _returnvalue _maxhealth)
        (set `/Game/FirstPersonBP/Blueprints/FirstPersonCharacter.Health` _maxhealth _asfirst_person_character)
        ;[1 1 1] Set New Ammo Count Text
        (if (and (`self.Level2UpgradeIsAmmunition`) (`self.AmmoSkipReady`))
          (set `self.AmmoSkipReady` false)
          (else
            (set `self.AmmoSkipReady` true)
            (`/Engine/EditorBlueprintResources/StandardMacros.DecrementInt` _currentammocount_2
              (:`  `
                (`TextRenderComponent.K2_SetText` (`self.AmmoCount`) (`KismetTextLibrary.Conv_IntToText` _currentammocount_2))))))
        (else
          (set `/Game/FirstPersonBP/Blueprints/FirstPersonCharacter.Health` _returnvalue _asfirst_person_character)
          (if (and (`self.Level2UpgradeIsAmmunition`) (`self.AmmoSkipReady`))
            (set `self.AmmoSkipReady` false)
            (else
              (set `self.AmmoSkipReady` true)
              (`/Engine/EditorBlueprintResources/StandardMacros.DecrementInt` _currentammocount
                (:`  `
                  (`TextRenderComponent.K2_SetText` (`self.AmmoCount`) (`KismetTextLibrary.Conv_IntToText` _currentammocount)))))))))))

(fn `UserConstructionScript`)
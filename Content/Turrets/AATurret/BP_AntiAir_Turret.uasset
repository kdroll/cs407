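; Anti-air turret that spots living flying enemies with pawn sensing and aims at the nearest tracked one, rotating gun and base separately.
; While enabled and loaded, it fires projectiles from top then bottom barrel with muzzle flashes, using delays and a firing flag to pace shots.
; Upgrade flags add damage, ricochet, sight range or halved ammo use.
; Floating text shows remaining ammo and turns to face the player.
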(event `self.ReceiveBeginPlay`
  ;[1 1 1] Ammo Count Initialization
  (set `self.Current Ammo Count` 75)
  (`TextRenderComponent.K2_SetText` (`self.AmmoCount`) (`KismetTextLibrary.Conv_IntToText` (`self.Current Ammo Count`))))

(event `self.PawnSensing.OnSeePawn`
  (params (Pawn :type "Pawn Object Reference"))
  (bind _enemies_in_range (`self.Enemies In Range`))
  (bind _aaturretturnableonly (`self.aaturretturnableonly`))
  (bind _aaturretgunonly (`self.aaturretgunonly`))
  ;[1 1 1] Aiming Logic
  (if (not (`self.Disabled`))
    (bind _asflying_enemy (cast `/Game/TestEnemies/FlyingEnemy/FlyingEnemy` Pawn))
    (set `self.TargetIsDead` (`/Game/TestEnemies/FlyingEnemy/FlyingEnemy.IsDead` _asflying_enemy))
    (if (not (`self.TargetIsDead`))
      (if (not (`KismetArrayLibrary.Array_Contains` (`self.Enemies In Range`) Pawn))
        (`KismetArrayLibrary.Array_Add` _enemies_in_range Pawn))
      (bind _returnednearestenemy (`self.GetNearestEnemy` _enemies_in_range))
      (bind _returnvalue (`self.K2_GetActorLocation` _returnednearestenemy))
      ;;[1 1 1] Set Gun Rotation
      (`SceneComponent.K2_SetWorldRotation` _aaturretgunonly (`KismetMathLibrary.MakeRotator` (.roll (`KismetMathLibrary.FindLookAtRotation` (`SceneComponent.K2_GetComponentLocation` _aaturretgunonly) _returnvalue)) (.pitch (`KismetMathLibrary.FindLookAtRotation` (`SceneComponent.K2_GetComponentLocation` _aaturretgunonly) _returnvalue)) (.yaw (`KismetMathLibrary.FindLookAtRotation` (`SceneComponent.K2_GetComponentLocation` _aaturretgunonly) _returnvalue))) false false)
      ;;[1 1 1] Set Gun Base Rotation
      (`SceneComponent.K2_SetWorldRotation` _aaturretturnableonly (`KismetMathLibrary.MakeRotator` 0.0 0.0 (.yaw (`KismetMathLibrary.FindLookAtRotation` (`SceneComponent.K2_GetComponentLocation` _aaturretturnableonly) _returnvalue))) false false)
      (if (not (`self.CurrentlyFiring`))
        (`self.Shootenemy` _returnednearestenemy)))))

(event `ShootEnemy`
  (params (Enemy :type "Pawn Object Reference"))
  ;[1 1 1] Shooting Logic
  (if (`self.Disabled`)
    _
    (elif (> (`self.Current Ammo Count`) 0)
      (set `self.CurrentlyFiring` true)
      (`|SpawnActorFromClass` "/Game/Turrets/AATurret/Projectile/AntiAirProjectile.AntiAirProjectile_C" (`SceneComponent.GetSocketTransform` (`self.aaturretgunonly`) "TopBarrel" "RTS_World") "AlwaysSpawn" "OverrideRootScale" null (`self.Level2UpgradeIsDamage`) (`self.Level3UpgradeIsRicochetBullets`))
      (`GameplayStatics.SpawnEmitterAtLocation` "/Game/InfinityBladeEffects/Effects/FX_Monsters/FX_Monster_Gruntling/Master/LaserMuzzleFlash.LaserMuzzleFlash" (`SceneComponent.GetSocketLocation` (`self.aaturretgunonly`) "TopBarrelEffect"))
      (`KismetSystemLibrary.Delay` (`self.TimeBetweenShots`))
      (`|SpawnActorFromClass` "/Game/Turrets/AATurret/Projectile/AntiAirProjectile.AntiAirProjectile_C" (`SceneComponent.GetSocketTransform` (`self.aaturretgunonly`) "BottomBarrel" "RTS_World") "AlwaysSpawn" "OverrideRootScale" null (`self.Level2UpgradeIsDamage`) (`self.Level3UpgradeIsRicochetBullets`))
      (`GameplayStatics.SpawnEmitterAtLocation` "/Game/InfinityBladeEffects/Effects/FX_Monsters/FX_Monster_Gruntling/Master/LaserMuzzleFlash.LaserMuzzleFlash" (`SceneComponent.GetSocketLocation` (`self.aaturretgunonly`) "BottomBarrelEffect"))
      (`KismetSystemLibrary.Delay` (`self.FireInterval`))
      (if (and (`self.Level2UpgradeIsAmmunition`) (`self.AmmoSkipReady`))
        (set `self.AmmoSkipReady` false)
        (else
          (`/Engine/EditorBlueprintResources/StandardMacros.DecrementInt` (`self.Current Ammo Count`)
            (:`  `
              (`TextRenderComponent.K2_SetText` (`self.AmmoCount`) (`KismetTextLibrary.Conv_IntToText` (`self.Current Ammo Count`)))
              (set `self.AmmoSkipReady` true)))))
      (set `self.CurrentlyFiring` false))))

(event `self.ReceiveTick`
  (params (DeltaSeconds :type "Float (single-precision)"))
  (bind _ammocount (`self.AmmoCount`))
  ;[1 1 1] Ammo Count Display Logic
  (`SceneComponent.K2_SetWorldRotation` _ammocount (`KismetMathLibrary.MakeRotator` 0.0 0.0 (.yaw (`KismetMathLibrary.FindLookAtRotation` (`SceneComponent.K2_GetComponentLocation` _ammocount) (`self.K2_GetActorLocation` (`GameplayStatics.GetPlayerCharacter` 0))))) false false)
  ;[1 1 1] Check for Range Upgrade
  (if (`self.Level2UpgradeIsRange`)
    (set `PawnSensingComponent.SightRadius` 3600.0 (`self.PawnSensing`))))

(fn `GetNearestEnemy`
  (params (EnemiesInRange :type "Array of Pawn Object Reference"))
  (returns (ReturnedNearestEnemy :type "Pawn Object Reference"))
  (set `self.ShortestDistance` 100000000.0)
  (for (_array_element _array_index) EnemiesInRange
    (`/Engine/EditorBlueprintResources/StandardMacros.IsValid` _array_element
      (:`Is Valid`
        (bind _returnvalue (`self.GetDistanceTo` _array_element))
        (if (< _returnvalue (`self.ShortestDistance`))
          (set `self.ShortestDistance` _returnvalue)
          (set `self.NearestEnemy` _array_element)))
      (:`Is Not Valid`
        (`KismetArrayLibrary.Array_Remove` EnemiesInRange _array_index))))
  (return (`self.NearestEnemy`)))

(fn `UserConstructionScript`)
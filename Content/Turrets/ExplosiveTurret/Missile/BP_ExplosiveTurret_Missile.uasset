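; Homing missile for the explosive turret that explodes on first overlap or after a short lifetime, with impulse and particles.
; Explosions deal splash damage to Enemy and EnemyTroll actors in radius, while the one hit takes direct damage.
; Homing starts weak as a delayed MultiGate chain repeatedly spawns dummy targets at the target's position, then jumps to strong acceleration.
; If the target becomes invalid, the missile homes on the last dummy.
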(event `self.ReceiveTick`
  (params (DeltaSeconds :type "Float (single-precision)"))
  (bind _projectile (`self.Projectile`))
  ;[1 1 1] Ensure Target is valid every tick
  (if (`ProjectileMovementComponent.bIsHomingProjectile` _projectile)
    (`/Engine/EditorBlueprintResources/StandardMacros.IsValid` (`ProjectileMovementComponent.HomingTargetComponent` _projectile)
      (:`Is Not Valid`
        (set `ProjectileMovementComponent.HomingTargetComponent` (`self.K2_GetRootComponent` (`self.DummyTargetReference`)) _projectile)))))

(event `self.ReceiveBeginPlay`
  ;[1 1 1] Ensure Missile doesn't live forever
  (`KismetSystemLibrary.Delay` 3.0)
  (`self.EmitImpulseAndEmitter`)
  (`self.SplashDamage` null)
  (`self.K2_DestroyActor`))

(event `self.CollisionComponent.OnComponentBeginOverlap`
  (params (OverlappedComponent :type "PrimitiveComponent Object Reference") (OtherActor :type "Actor Object Reference") (OtherComp :type "PrimitiveComponent Object Reference") (OtherBodyIndex :type Integer) (bFromSweep :type Boolean) (SweepResult :type "HitResult Structure (by ref)"))
  ;[1 1 1] Explode on Contact
  (`/Engine/EditorBlueprintResources/StandardMacros.DoOnce` false
    (:`Completed`
      (`self.EmitImpulseAndEmitter`)
      (`self.SplashDamage` OtherActor)
      (bind _asenemy (cast `/Game/TestEnemies/Enemy` OtherActor)
        (:`then`
          (`/Game/TestEnemies/Enemy.TakeDamage` _asenemy (`KismetMathLibrary.Conv_IntToDouble` (`self.DamageValue`)) false)
          (`self.K2_DestroyActor`))
        (:`CastFailed`
          (bind _asenemy_troll (cast `/Game/TestEnemies/EnemyTroll` OtherActor)
            (:`then`
              (`/Game/TestEnemies/EnemyTroll.TakeDamage` _asenemy_troll (`KismetMathLibrary.Conv_IntToDouble` (`self.DamageValue`)) false)
              (`self.K2_DestroyActor`))
            (:`CastFailed`
              (`self.EmitImpulseAndEmitter`)
              (`self.K2_DestroyActor`))))))))

(event `CallMultiGate`
  (bind _originaltargetreference (`self.OriginalTargetReference`))
  (bind _originaltargetreference_2 (`self.OriginalTargetReference`))
  (bind _projectile (`self.Projectile`))
  (bind _projectile_2 (`self.Projectile`))
  (bind _originaltargetreference_3 (`self.OriginalTargetReference`))
  (bind _originaltargetreference_4 (`self.OriginalTargetReference`))
  (bind _originaltargetreference_5 (`self.OriginalTargetReference`))
  ;[1 1 1] Update Dummy Target
  (`|MultiGate` false
    (:`Out 0`
      (`KismetSystemLibrary.Delay` 0.2)
      (`/Engine/EditorBlueprintResources/StandardMacros.IsValid` _originaltargetreference
        (:`Is Valid`
          (`self.SpawnNewDummyTarget` _originaltargetreference)
          (`self.CallMultiGate`))
        (:`Is Not Valid`
          (set `self.NewTargetIsSet` true)
          (`self.CallMultiGate`))))
    (:`Out 1`
      (`KismetSystemLibrary.Delay` 0.2)
      (if (`self.NewTargetIsSet`)
        (`self.CallMultiGate`)
        (else
          (`/Engine/EditorBlueprintResources/StandardMacros.IsValid` _originaltargetreference_3
            (:`Is Valid`
              (`self.SpawnNewDummyTarget` _originaltargetreference_3)
              (`self.CallMultiGate`))
            (:`Is Not Valid`
              (set `self.NewTargetIsSet` true)
              (`self.CallMultiGate`))))))
    (:`Out 2`
      (`KismetSystemLibrary.Delay` 0.2)
      (if (`self.NewTargetIsSet`)
        (`self.CallMultiGate`)
        (else
          (`/Engine/EditorBlueprintResources/StandardMacros.IsValid` _originaltargetreference_4
            (:`Is Valid`
              (`self.SpawnNewDummyTarget` _originaltargetreference_4)
              (`self.CallMultiGate`))
            (:`Is Not Valid`
              (set `self.NewTargetIsSet` true)
              (`self.CallMultiGate`))))))
    (:`Out 3`
      (`KismetSystemLibrary.Delay` 0.2)
      (if (`self.NewTargetIsSet`)
        (`self.CallMultiGate`)
        (else
          (`/Engine/EditorBlueprintResources/StandardMacros.IsValid` _originaltargetreference_5
            (:`Is Valid`
              (`self.SpawnNewDummyTarget` _originaltargetreference_5)
              (`self.CallMultiGate`))
            (:`Is Not Valid`
              (set `self.NewTargetIsSet` true)
              (`self.CallMultiGate`))))))
    (:`Out 4`
      (`KismetSystemLibrary.Delay` 0.2)
      (if (`self.NewTargetIsSet`)
        (`self.CallMultiGate`)
        (else
          (`/Engine/EditorBlueprintResources/StandardMacros.IsValid` _originaltargetreference_2
            (:`Is Valid`
              (`self.SpawnNewDummyTarget` _originaltargetreference_2)
              (`self.CallMultiGate`))
            (:`Is Not Valid`
              (set `self.NewTargetIsSet` true)
              (`self.CallMultiGate`))))))
    (:`Out 5`
      (if (`self.NewTargetIsSet`)
        (set `ProjectileMovementComponent.HomingTargetComponent` (`self.K2_GetRootComponent` (`self.DummyTargetReference`)) _projectile)
        (set `ProjectileMovementComponent.HomingAccelerationMagnitude` 40000.0 _projectile)
        (else
          (set `ProjectileMovementComponent.HomingTargetComponent` (`self.K2_GetRootComponent` (`self.OriginalTargetReference`)) _projectile_2)
          (set `ProjectileMovementComponent.HomingAccelerationMagnitude` 40000.0 _projectile_2))))))

(event `HomeInOnTarget`
  (params (TargetToHomeTo :type "Actor Object Reference"))
  (bind _projectile (`self.Projectile`))
  ;[1 1 1] Set Homing
  (bind _output_get (set `self.OriginalTargetReference` TargetToHomeTo))
  (`self.SpawnNewDummyTarget` _output_get)
  (set `ProjectileMovementComponent.HomingTargetComponent` (`self.K2_GetRootComponent` (`self.OriginalTargetReference`)) _projectile)
  (set `ProjectileMovementComponent.bIsHomingProjectile` true _projectile)
  (set `ProjectileMovementComponent.HomingAccelerationMagnitude` 1.0 _projectile)
  (`self.CallMultiGate`))

(fn `EmitImpulseAndEmitter`
  (bind _explosionforce (`self.ExplosionForce`))
  (`RadialForceComponent.FireImpulse` _explosionforce)
  (`GameplayStatics.SpawnEmitterAtLocation` "/Game/InfinityBladeEffects/Effects/FX_Monsters/FX_Monster_Gruntling/Bomber/P_FireBombExplosion.P_FireBombExplosion" (`SceneComponent.K2_GetComponentLocation` _explosionforce)))

(fn `SpawnNewDummyTarget`
  (params (ActorToSpawnAt :type "Actor Object Reference"))
  (bind _returnvalue (`|SpawnActorFromClass` "/Game/Turrets/ExplosiveTurret/Missile/BP_HomingTarget.BP_HomingTarget_C" (`KismetMathLibrary.MakeTransform` (`KismetMathLibrary.MakeVector` (.x (.location (`self.GetTransform` ActorToSpawnAt))) (.y (.location (`self.GetTransform` ActorToSpawnAt))) (- (.z (.location (`self.GetTransform` ActorToSpawnAt))) 20.0)) (.rotation (`self.GetTransform` ActorToSpawnAt)) (.scale (`self.GetTransform` ActorToSpawnAt))) "Undefined" "OverrideRootScale"))
  (set `self.DummyTargetReference` _returnvalue))

(fn `SplashDamage`
  (params (OriginalHitActor :type "Actor Object Reference"))
  (for _array_element (`PrimitiveComponent.GetOverlappingActors` (`self.ExplosionRadius`) null)
    (if (not (== OriginalHitActor _array_element))
      (bind _asenemy (cast `/Game/TestEnemies/Enemy` _array_element)
        (:`then`
          (`/Game/TestEnemies/Enemy.TakeDamage` _asenemy (`KismetMathLibrary.Conv_IntToDouble` (`self.SplashDamageValue`)) false))
        (:`CastFailed`
          (bind _asenemy_troll (cast `/Game/TestEnemies/EnemyTroll` _array_element))
          (`/Game/TestEnemies/EnemyTroll.TakeDamage` _asenemy_troll (`KismetMathLibrary.Conv_IntToDouble` (`self.SplashDamageValue`)) false))))))

(fn `UserConstructionScript`)
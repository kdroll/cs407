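; Explosive turret that detects Enemy and EnemyTroll pawns through PawnSensing and fires homing missiles at the nearest one.
; Each sighting adds to a tracked list, which is pruned only of invalid entries, then yaws the model toward the closest target.
; Firing spawns a missile and muzzle flash at the barrel socket, limited by ammo, a fire-interval delay and a Disabled flag.
; A floating ammo counter turns to face the player every tick.
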(event `self.ReceiveBeginPlay`
  ;[1 1 1] Ammo Count Initialization
  (set `self.CurrentAmmoCount` 2000)
  (`TextRenderComponent.K2_SetText` (`self.AmmoCount`) (`KismetTextLibrary.Conv_IntToText` (`self.CurrentAmmoCount`))))

(event `self.PawnSensing.OnSeePawn`
  (params (Pawn :type "Pawn Object Reference"))
  (bind _turretmodel (`self.TurretModel`))
  (bind _enemiesinrange (`self.EnemiesInRange`))
  ;[1 1 1] Aiming Logic
  (if (not (`self.Disabled`))
    (cast `/Game/TestEnemies/Enemy` Pawn
      (:`then`
        _)
      (:`CastFailed`
        (cast `/Game/TestEnemies/EnemyTroll` Pawn)))
    (if (not (`KismetArrayLibrary.Array_Contains` (`self.EnemiesInRange`) Pawn))
      (`KismetArrayLibrary.Array_Add` _enemiesinrange Pawn))
    (bind _returnedclosestenemy (`self.GetNearestEnemy` _enemiesinrange))
    (`/Engine/EditorBlueprintResources/StandardMacros.IsValid` _returnedclosestenemy
      (:`Is Valid`
        (`SceneComponent.K2_SetWorldRotation` _turretmodel (`KismetMathLibrary.MakeRotator` (.roll (`SceneComponent.K2_GetComponentRotation` _turretmodel)) (.pitch (`SceneComponent.K2_GetComponentRotation` _turretmodel)) (.yaw (`KismetMathLibrary.FindLookAtRotation` (`SceneComponent.K2_GetComponentLocation` _turretmodel) (`self.K2_GetActorLocation` _returnedclosestenemy)))) false false)
        (if (not (`self.CurrentlyFiring`))
          (`self.Shootenemy` _returnedclosestenemy))))))

(event `ShootEnemy`
  (params (Enemy :type "Pawn Object Reference"))
  ;[1 1 1] Shooting Logic
  (if (`self.Disabled`)
    _
    (elif (> (`self.CurrentAmmoCount`) 0)
      (set `self.CurrentlyFiring` true)
      (bind _returnvalue (`|SpawnActorFromClass` "/Game/Turrets/ExplosiveTurret/Missile/BP_ExplosiveTurret_Missile.BP_ExplosiveTurret_Missile_C" (`SceneComponent.GetSocketTransform` (`self.TurretModel`) "MainBarrel" "RTS_World") "AdjustIfPossibleButAlwaysSpawn" "OverrideRootScale"))
      (`/Game/Turrets/ExplosiveTurret/Missile/BP_ExplosiveTurret_Missile.HomeInOnTarget` _returnvalue Enemy)
      (`GameplayStatics.SpawnEmitterAtLocation` "/Game/InfinityBladeEffects/Effects/FX_Monsters/FX_Monster_Gruntling/Master/LaserMuzzleFlash.LaserMuzzleFlash" (`SceneComponent.GetSocketLocation` (`self.TurretModel`) "MainBarrel"))
      (`/Engine/EditorBlueprintResources/StandardMacros.DecrementInt` (`self.CurrentAmmoCount`)
        (:`  `
          (`TextRenderComponent.K2_SetText` (`self.AmmoCount`) (`KismetTextLibrary.Conv_IntToText` (`self.CurrentAmmoCount`)))
          (`KismetSystemLibrary.Delay` (`self.FireInterval`))
          (set `self.CurrentlyFiring` false))))))

(event `self.ReceiveTick`
  (params (DeltaSeconds :type "Float (single-precision)"))
  (bind _ammocount (`self.AmmoCount`))
  ;[1 1 1] Ammo Count Display
  (`SceneComponent.K2_SetWorldRotation` _ammocount (`KismetMathLibrary.MakeRotator` 0.0 0.0 (.yaw (`KismetMathLibrary.FindLookAtRotation` (`SceneComponent.K2_GetComponentLocation` _ammocount) (`self.K2_GetActorLocation` (`GameplayStatics.GetPlayerCharacter` 0))))) false false))

(fn `GetNearestEnemy`
  (params (EnemiesInRange :type "Array of Pawn Object Reference"))
  (returns (ReturnedClosestEnemy :type "Pawn Object Reference"))
  (set `self.ShortestDistance` 100000000.0)
  (for (_array_element _array_index) EnemiesInRange
    (`/Engine/EditorBlueprintResources/StandardMacros.IsValid` _array_element
      (:`Is Valid`
        (bind _returnvalue (`self.GetDistanceTo` _array_element))
        (if (< _returnvalue (`self.ShortestDistance`))
          (set `self.ShortestDistance` _returnvalue)
          (set `self.ClosestEnemy` _array_element)))
      (:`Is Not Valid`
        (`KismetArrayLibrary.Array_Remove` EnemiesInRange _array_index))))
  (return (`self.ClosestEnemy`)))

(fn `UserConstructionScript`)
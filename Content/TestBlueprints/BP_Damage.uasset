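; BP_Damage is a damage number actor that shows DamageAmount as text, set on its TextRender in the construction script.
; On BeginPlay it stores its start location and plays a timeline that sets its height offset and text size while rotating it to face the player pawn.
; The actor destroys itself when the timeline finishes.
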(event `self.ReceiveBeginPlay`
  (bind (_startinglocation_x _startinglocation_y _startinglocation_z) (`KismetMathLibrary.BreakVector` (`self.StartingLocation`)))
  (set `self.StartingLocation` (`self.K2_GetActorLocation`))
  (`Timeline|Timeline_0`
    (:`Update`
      (`self.K2_SetActorLocationAndRotation` (`KismetMathLibrary.MakeVector` _startinglocation_x _startinglocation_y (+ _startinglocation_z (* 0.0 100.0))) (`KismetMathLibrary.FindLookAtRotation` (`self.K2_GetActorLocation`) (`self.K2_GetActorLocation` (`GameplayStatics.GetPlayerPawn` 0))))
      (`TextRenderComponent.SetWorldSize` (`self.TextRender`) (* 0.0 (`self.Font Size`))))
    (:`Finished`
      (`self.K2_DestroyActor`))))

(fn `UserConstructionScript`
  (`TextRenderComponent.K2_SetText` (`self.TextRender`) (`KismetTextLibrary.Conv_IntToText` (`self.Damage Amount`))))